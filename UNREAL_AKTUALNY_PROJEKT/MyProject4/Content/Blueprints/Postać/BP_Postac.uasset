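; BP_Postac is the player character, with movement, jump, crouch, health and a Glock.
; Weapon switch, attack and reload functions branch on the current weapon; Glock shots use camera line traces to apply damage, with persistent debug drawing.
; Lethal damage teleports the character to a fixed point and restores health.
; Left click and Space emit MakeNoise events, and getter functions expose health, ammo and magazine size.
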(event `self.ReceiveAnyDamage`
  (params (Damage :type "Float (single-precision)") (DamageType :type "DamageType Object Reference") (InstigatedBy :type "Controller Object Reference") (DamageCauser :type "Actor Object Reference"))
  ;[1 1 1] Obrażenia_Odradzanie
  (set `self.Zycie` (- (`self.Zycie`) Damage))
  (if (<= (`self.Zycie`) 0.0)
    (`self.K2_TeleportTo` (165.0 0.0 124.008842) (struct :`Yaw` 179.999756))
    (set `self.Zycie` (`self.Max_Zycie`))))

(event `Key|LeftMouseButton`
  (bind _returnvalue (`GameplayStatics.GetPlayerPawn` 0))
  ;[1 1 1] Hałasowanie
  (:`Pressed`
    (if (not (== 0 1))
      (`self.MakeNoise` 1.0 _returnvalue (`self.K2_GetActorLocation` _returnvalue) :!label _label))))

(event `Key|SpaceBar`
  ;[1 1 1] Hałasowanie
  (:`Pressed`
    (`GameplayStatics.PlaySoundAtLocation` null (`self.K2_GetActorLocation` (`GameplayStatics.GetPlayerPawn` 0)))
    (goto _label)))

(event `InputAxis|Ruch_Przod_Tyl`
  (params (AxisValue :type "Float (single-precision)"))
  ;[1 1 1] Ruch_Postaci
  ;;[1 1 1] Klawiatura Ruch
  (`self.AddMovementInput` (`KismetMathLibrary.GetForwardVector` (`KismetMathLibrary.MakeRot` 0.0 (.yaw (`self.GetControlRotation`)))) AxisValue))

(event `InputAxis|Ruch_Prawo_Lewo`
  (params (AxisValue :type "Float (single-precision)"))
  ;[1 1 1] Ruch_Postaci
  ;;[1 1 1] Klawiatura Ruch
  (`self.AddMovementInput` (`KismetMathLibrary.GetRightVector` (`KismetMathLibrary.MakeRot` 0.0 (.yaw (`self.GetControlRotation`)))) AxisValue))

(event `InputAction|Glock`
  ;[1 1 1] Obsługa Broni
  (:`Pressed`
    (`self.Zmiana_Broni` "NewEnumerator1")))

(event `InputAction|Skok`
  ;[1 1 1] Ruch_Postaci
  ;;[1 1 1] Skok
  (:`Pressed`
    (`self.Jump`)))

(event `InputAxis|Widok_Prawa_Lewa`
  (params (AxisValue :type "Float (single-precision)"))
  ;[1 1 1] Ruch_Postaci
  ;;[1 1 1] Mysz Ruch
  (`self.AddControllerYawInput` AxisValue))

(event `InputAxis|Widok_Gor_Dol`
  (params (AxisValue :type "Float (single-precision)"))
  ;[1 1 1] Ruch_Postaci
  ;;[1 1 1] Mysz Ruch
  (`self.AddControllerPitchInput` AxisValue))

(event `InputAction|Atak`
  ;[1 1 1] Obsługa Broni
  (:`Pressed`
    (`self.Atak`)))

(event `InputAction|Kucanie`
  ;[1 1 1] Ruch_Postaci
  ;;[1 1 1] Kucanie
  (:`Pressed`
    (`self.Crouch`))
  (:`Released`
    (`self.UnCrouch`)))

(event `InputAction|Przeładuj`
  ;[1 1 1] Obsługa Broni
  (:`Pressed`
    (`self.Przeladowanie`)))

(fn `Amunicja_glock`
  (returns (Aktualna_Amunicja :type Integer))
  (return (`self.glock_amunicja`)))

(fn `Atak`
  (switch `/Game/Blueprints/Mechanika/Spis_Broni` (`self.Aktualna_Bron`)
    (:`NewEnumerator1`
      (`self.Glock`))))

(fn `Glock`
  (bind _camera1 (`self.Camera1`))
  (bind _glock_amunicja (`self.glock_amunicja`))
  (bind _returnvalue (`SceneComponent.K2_GetComponentLocation` _camera1))
  (if (== _glock_amunicja 0)
    (`KismetSystemLibrary.PrintString` "Przeladuj!")
    (else
      (set `self.glock_amunicja` (- _glock_amunicja 1))
      (`GameplayStatics.PlaySoundAtLocation` "/Game/Audio/Broń/Glock/glock18-1.glock18-1")
      (bind (_outhit _returnvalue_2) (`KismetSystemLibrary.LineTraceSingle` :`Start` _returnvalue :`End` (+ (* (`SceneComponent.GetForwardVector` _camera1) 500.0) _returnvalue) :`TraceChannel` "TraceTypeQuery2" :`bTraceComplex` true :`DrawDebugType` "Persistent"))
      (if _returnvalue_2
        (`GameplayStatics.ApplyDamage` (`.HitActor` (`GameplayStatics.BreakHitResult` _outhit)) 50.0)))))

(fn `hp`
  (returns (`Aktualne HP` :type "Float (double-precision)") (`Maksymalne HP` :type "Float (double-precision)"))
  (return (`self.Zycie`) (`self.Max_Zycie`)))

(fn `Magazynek_glock`
  (returns (Pojemnosc_Magazynka :type Integer))
  (return (`self.glock_max_amunicja`)))

(fn `Przeladowanie`
  (bind _glock_zapas_amunicji (`self.glock_zapas_amunicji`))
  (bind _glock_amunicja (`self.glock_amunicja`))
  (bind _returnvalue (- (`self.glock_max_amunicja`) _glock_amunicja))
  (bind _returnvalue_2 (+ _returnvalue (`self.glock_amunicja`) 0))
  (switch `/Game/Blueprints/Mechanika/Spis_Broni` (`self.Aktualna_Bron`)
    (:`NewEnumerator1`
      (if (and (< (`self.glock_amunicja`) (`self.glock_max_amunicja`)) (> (`self.glock_zapas_amunicji`) 0))
        (`GameplayStatics.PlaySoundAtLocation` "/Game/Audio/Broń/Glock/glock_reload_sound.glock_reload_sound")
        (`SkeletalMeshComponent.PlayAnimation` (`self.SkeletalMesh1`) "/Game/Animations/Reload_Pistol.Reload_Pistol" false)
        (if (> _returnvalue _glock_zapas_amunicji)
          (set `self.glock_amunicja` (+ _glock_zapas_amunicji _glock_amunicja))
          (set `self.glock_zapas_amunicji` 0)
          (else
            (set `self.glock_amunicja` _returnvalue_2)
            (set `self.glock_zapas_amunicji` (- (`self.glock_zapas_amunicji`) _returnvalue_2))))))))

(fn `UserConstructionScript`)

(fn `Zmiana_Broni`
  (params (Spis_Broni :type "/Game/Blueprints/Mechanika/Spis_Broni Enum" :default "NewEnumerator0"))
  (bind _bron (`self.bron`))
  (switch `/Game/Blueprints/Mechanika/Spis_Broni` Spis_Broni
    (:`NewEnumerator1`
      (`StaticMeshComponent.SetStaticMesh` _bron "/Game/Broń/glock.Glock")
      (`SceneComponent.AttachTo` _bron (`self.SkeletalMesh1`) "E" "KeepRelativeOffset")
      (set `self.Aktualna_Bron` "NewEnumerator1"))))