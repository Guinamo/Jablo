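; BP_Wrog1 is an enemy with hit points that hands a target to its AI and is destroyed when its health runs out.
; On BeginPlay it writes its Target variable into the AITarget1 blackboard key.
; AnyDamage subtracts damage from Hp, prints the remaining value and destroys the actor at zero or below.
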(event `self.ReceiveAnyDamage`
  (params (Damage :type "Float (single-precision)") (DamageType :type "DamageType Object Reference") (InstigatedBy :type "Controller Object Reference") (DamageCauser :type "Actor Object Reference"))
  (bind _hp (`self.hp`))
  (set `self.hp` (- (`self.hp`) Damage))
  (`KismetSystemLibrary.PrintString` (`KismetStringLibrary.Conv_DoubleToString` _hp))
  (if (<= _hp 0.0)
    (`self.K2_DestroyActor`)))

(event `self.ReceiveBeginPlay`
  (`BlackboardComponent.SetValueAsObject` (`AIBlueprintHelperLibrary.GetBlackboard` self) "AITarget1" (`self.Target`)))

(fn `UserConstructionScript`)