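; BP_Postac is a player character with movement, mouse look, jumping and four weapons: knife, Glock, shotgun and Uzi.
; Weapon keys swap static meshes and set WybranaBron, which selects the attack and reload branches.
; Attacks apply damage via debug-drawn camera line traces, with the Uzi looping through a Gate and RetriggerableDelay while held.
; Glock and Uzi spend ammo; the shotgun fires without checking it, though reload refills all three guns' counters after a delay, one per selected gun.
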(event `InputAxis|Ruch_Przod_Tyl`
  (params (AxisValue :type "Float (single-precision)"))
  ;[1 1 1] Ruch_Postaci
  ;;[1 1 1] Klawiatura Ruch
  (`self.AddMovementInput` (`KismetMathLibrary.GetForwardVector` (`KismetMathLibrary.MakeRot` 0.0 (.yaw (`self.GetControlRotation`)))) AxisValue))

(event `InputAxis|Ruch_Prawo_Lewo`
  (params (AxisValue :type "Float (single-precision)"))
  ;[1 1 1] Ruch_Postaci
  ;;[1 1 1] Klawiatura Ruch
  (`self.AddMovementInput` (`KismetMathLibrary.GetRightVector` (`KismetMathLibrary.MakeRot` 0.0 (.yaw (`self.GetControlRotation`)))) AxisValue))

(event `InputAction|Skok`
  ;[1 1 1] Ruch_Postaci
  ;;[1 1 1] Skok
  (:`Pressed`
    (`self.Jump`)))

(event `InputAxis|Widok_Prawa_Lewa`
  (params (AxisValue :type "Float (single-precision)"))
  ;[1 1 1] Ruch_Postaci
  ;;[1 1 1] Mysz Ruch
  (`self.AddControllerYawInput` AxisValue))

(event `InputAction|Nóż`
  ;[1 1 1] Obsługa Broni
  ;;[1 1 1] Wybór_Broni
  (:`Pressed`
    (`StaticMeshComponent.SetStaticMesh` (`self.noz`) "/Game/Broń/knife.knife")
    (`StaticMeshComponent.SetStaticMesh` (`self.Uzi`) null)
    (`StaticMeshComponent.SetStaticMesh` (`self.Glock`) null)
    (`StaticMeshComponent.SetStaticMesh` (`self.dubeltowka`) null)
    (set `self.Wybrana_Bron` 1)))

(event `InputAction|Glock`
  ;[1 1 1] Obsługa Broni
  ;;[1 1 1] Wybór_Broni
  (:`Pressed`
    (`StaticMeshComponent.SetStaticMesh` (`self.Glock`) "/Game/Broń/glock.Glock")
    (`StaticMeshComponent.SetStaticMesh` (`self.noz`) null)
    (`StaticMeshComponent.SetStaticMesh` (`self.dubeltowka`) null)
    (`StaticMeshComponent.SetStaticMesh` (`self.Uzi`) null)
    (set `self.Wybrana_Bron` 2)))

(event `InputAxis|Widok_Gor_Dol`
  (params (AxisValue :type "Float (single-precision)"))
  ;[1 1 1] Ruch_Postaci
  ;;[1 1 1] Mysz Ruch
  (`self.AddControllerPitchInput` AxisValue))

(event `InputAction|dubeltówka`
  ;[1 1 1] Obsługa Broni
  ;;[1 1 1] Wybór_Broni
  (:`Pressed`
    (`StaticMeshComponent.SetStaticMesh` (`self.dubeltowka`) "/Game/Broń/dubeltowka.dubeltowka")
    (`StaticMeshComponent.SetStaticMesh` (`self.noz`) null)
    (`StaticMeshComponent.SetStaticMesh` (`self.Glock`) null)
    (`StaticMeshComponent.SetStaticMesh` (`self.Uzi`) null)
    (set `self.Wybrana_Bron` 3)))

(event `InputAction|Uzi`
  ;[1 1 1] Obsługa Broni
  ;;[1 1 1] Wybór_Broni
  (:`Pressed`
    (`StaticMeshComponent.SetStaticMesh` (`self.Uzi`) "/Game/Broń/uzi.Uzi")
    (`StaticMeshComponent.SetStaticMesh` (`self.noz`) null)
    (`StaticMeshComponent.SetStaticMesh` (`self.Glock`) null)
    (`StaticMeshComponent.SetStaticMesh` (`self.dubeltowka`) null)
    (set `self.Wybrana_Bron` 4)))

(event `InputAction|Przeładuj`
  ;[1 1 1] Obsługa Broni
  ;;[1 1 1] Przeładowanie
  (:`Pressed`
    (if (== (`self.Wybrana_Bron`) 1)
      _
      (elif (== (`self.Wybrana_Bron`) 2)
        (`KismetSystemLibrary.Delay` 5.0)
        (set `self.Amunicja_2` (`self.Max_Amunicja_2`))
        (elif (== (`self.Wybrana_Bron`) 3)
          (`KismetSystemLibrary.Delay` 5.0)
          (set `self.Amunicja_3` (`self.Max_Amunicja_3`))
          (elif (== (`self.Wybrana_Bron`) 4)
            (`KismetSystemLibrary.Delay` 5.0)
            (set `self.Amunicja_4` (`self.Max_Amunicja_4`))))))))

(event `InputAction|Atak`
  (bind _camera1 (`self.Camera1`))
  (bind _wybrana_bron (`self.Wybrana_Bron`))
  (bind _camera1_2 (`self.Camera1`))
  (bind _camera1_3 (`self.Camera1`))
  (bind _camera1_4 (`self.Camera1`))
  (bind _returnvalue (`SceneComponent.K2_GetComponentLocation` _camera1))
  (bind _returnvalue_2 (`SceneComponent.K2_GetComponentLocation` _camera1_2))
  (bind _returnvalue_3 (`SceneComponent.K2_GetComponentLocation` _camera1_4))
  (bind _returnvalue_4 (`SceneComponent.K2_GetComponentLocation` _camera1_3))
  ;[1 1 1] Obsługa Broni
  ;;[1 1 1] Atak_oraz_Obrażenia
  (:`Pressed`
    (if (== _wybrana_bron 4)
      (`|ExecutionSequence`
        (:`then_0`
          (goto _label :!via `Open`))
        (:`then_1`
          (`/Engine/EditorBlueprintResources/StandardMacros.Gate` true :!label _label
            (:`Exit`
              (`|ExecutionSequence`
                (:`then_0`
                  (if (> (`self.Amunicja_4`) 0)
                    (bind (_outhit _returnvalue_5) (`KismetSystemLibrary.LineTraceSingle` :`Start` _returnvalue_2 :`End` (+ (* (`SceneComponent.GetForwardVector` _camera1_2) 500.0) _returnvalue_2) :`TraceChannel` "TraceTypeQuery2" :`bTraceComplex` true :`DrawDebugType` "Persistent"))
                    (set `self.Amunicja_4` (- (`self.Amunicja_4`) 1))
                    (if _returnvalue_5
                      (`GameplayStatics.ApplyDamage` (`.HitActor` (`GameplayStatics.BreakHitResult` _outhit)) 40.0))
                    (else
                      (`KismetSystemLibrary.PrintString` "Przeladuj" :!label _label_2))))
                (:`then_1`
                  (`KismetSystemLibrary.RetriggerableDelay` 0.2)
                  (goto _label)))))))
      (elif (== _wybrana_bron 1)
        (`KismetSystemLibrary.PrintString` "ciach")
        (bind (_outhit_2 _returnvalue_6) (`KismetSystemLibrary.LineTraceSingle` :`Start` _returnvalue :`End` (+ (* (`SceneComponent.GetForwardVector` _camera1) 70.0) _returnvalue) :`TraceChannel` "TraceTypeQuery2" :`bTraceComplex` true :`DrawDebugType` "Persistent"))
        (if _returnvalue_6
          (`GameplayStatics.ApplyDamage` (`.HitActor` (`GameplayStatics.BreakHitResult` _outhit_2)) 30.0))
        (elif (== _wybrana_bron 2)
          (if (> (`self.Amunicja_2`) 0)
            (`GameplayStatics.PlaySoundAtLocation` "/Game/Audio/Broń/glock18-1.glock18-1")
            (bind (_outhit_3 _returnvalue_7) (`KismetSystemLibrary.LineTraceSingle` :`Start` _returnvalue_3 :`End` (+ (* (`SceneComponent.GetForwardVector` _camera1_4) 500.0) _returnvalue_3) :`TraceChannel` "TraceTypeQuery2" :`bTraceComplex` true :`DrawDebugType` "Persistent"))
            (set `self.Amunicja_2` (- (`self.Amunicja_2`) 1))
            (if _returnvalue_7
              (`GameplayStatics.ApplyDamage` (`.HitActor` (`GameplayStatics.BreakHitResult` _outhit_3)) 50.0))
            (else
              (goto _label_2)))
          (elif (== _wybrana_bron 3)
            (`KismetSystemLibrary.PrintString` "bam")
            (bind (_outhit_4 _returnvalue_8) (`KismetSystemLibrary.LineTraceSingle` :`Start` _returnvalue_4 :`End` (+ (* (`SceneComponent.GetForwardVector` _camera1_3) 500.0) _returnvalue_4) :`TraceChannel` "TraceTypeQuery2" :`bTraceComplex` true :`DrawDebugType` "Persistent"))
            (if _returnvalue_8
              (`GameplayStatics.ApplyDamage` (`.HitActor` (`GameplayStatics.BreakHitResult` _outhit_4)) 70.0)))))))
  (:`Released`
    (goto _label :!via `Close`)))

(fn `UserConstructionScript`)