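; BP_Wrog1 is an enemy Blueprint with health that takes damage and is destroyed when its HP runs out.
; On BeginPlay it writes its Target variable into the AITarget1 key of its AI blackboard.
; AnyDamage passes HP and damage to OdejmijHP, which destroys the actor at zero or below and returns the remainder, which is then stored and printed.
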(event `self.ReceiveAnyDamage`
  (params (Damage :type "Float (single-precision)") (DamageType :type "DamageType Object Reference") (InstigatedBy :type "Controller Object Reference") (DamageCauser :type "Actor Object Reference"))
  (bind _hp (`self.hp`))
  (bind _hp_out (`self.odejmij_HP` _hp Damage))
  (set `self.hp` _hp_out)
  (`KismetSystemLibrary.PrintString` (`KismetStringLibrary.Conv_DoubleToString` _hp)))

(event `self.ReceiveBeginPlay`
  (`BlackboardComponent.SetValueAsObject` (`AIBlueprintHelperLibrary.GetBlackboard` self) "AITarget1" (`self.Target`)))

(fn `odejmij_HP`
  (params (HP_in :type "Float (double-precision)") (damage :type "Float (double-precision)"))
  (returns (HP_out :type "Float (double-precision)"))
  (bind _returnvalue (- HP_in damage))
  (if (<= _returnvalue 0.0)
    (`self.K2_DestroyActor`))
  (return _returnvalue))

(fn `UserConstructionScript`)