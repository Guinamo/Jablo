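; AI controller for enemies that runs the BT_AI_Wrog behavior tree on BeginPlay and feeds it sight and hearing input.
; A PawnSensing component writes any seen pawn to the blackboard as the enemy actor.
; Heard noises within a fixed distance of the controlled pawn store their location as a position to check and set a heard-something flag.
; The controller only sets these keys and never clears them.
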(event `self.ReceiveBeginPlay`
  (`self.RunBehaviorTree` "/Game/Blueprints/Mechanika/AI/BT_AI_Wrog.BT_AI_Wrog"))

(event `self.PawnSensing1.OnSeePawn`
  (params (Pawn :type "Pawn Object Reference"))
  (`BlackboardComponent.SetValueAsObject` (`AIBlueprintHelperLibrary.GetBlackboard` self) (`self.WrogActorKey`) Pawn))

(event `self.PawnSensing1.OnHearNoise`
  (params (Instigator :type "Pawn Object Reference") (Location :type "Object.Vector Structure (by ref)") (Volume :type "Float (single-precision)"))
  (bind _returnvalue (`AIBlueprintHelperLibrary.GetBlackboard` self))
  (if (< (`KismetMathLibrary.VSize` (- Location (`Pawn.GetNavAgentLocation` (`self.K2_GetPawn`)))) 900.0)
    (`BlackboardComponent.SetValueAsVector` _returnvalue (`self.sprawdzeniepozycjikey`) Location)
    (`BlackboardComponent.SetValueAsBool` _returnvalue (`self.uslyszalcosboolkey`) true)))

(fn `UserConstructionScript`)