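; Player character for a shooter, with movement, jump, crouch, noise emission, and health that resets with a teleport on death.
; Number keys or cycling set a slot index into parallel weapon arrays and swap the held mesh; slots past Uzi are knife placeholders.
; Firing runs debug-drawn camera traces with random spread and multiple shotgun pellets, looping through Delay for automatics.
; Reloading refills magazines from reserve ammo and blocks firing for a fixed delay.
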(event EventBeginPlay
  ;[1 1 1] Wybieranie broni
  (CallFunction|BronZmiana)
  ;[1 0.08657 0] Debug
  (Development|PrintString (Utilities|Array|Get(acopy) (Variables|Default|Getbron_nazwy) (Variables|Default|Getaktualna))))

(event EventAnyDamage
  (params (Damage :type Float%20%28single-precision%29) (DamageType :type Damage%20Type%20Object%20Reference) (InstigatedBy :type Controller%20Object%20Reference) (DamageCauser :type Actor%20Object%20Reference))
  ;[1 1 1] Obrażenia_Odradzanie
  (Variables|Default|SetZycie (- (Variables|Default|GetZycie) Damage))
  (if (<= (Variables|Default|GetZycie) 0.0)
    (Transformation|Teleport "165.000000, 0,124.008842" "0,179.999756, 0")
    (Variables|Default|SetZycie (Variables|Default|GetMax_Zycie))))

(event Input|ActionEvents|InputActionKucanie
  ;[1 1 1] Ruch_Postaci
  ;;[1 1 1] Kucanie
  (:Pressed
    (Character|Crouch))
  (:Released
    (Character|UnCrouch)))

(event Input|ActionEvents|InputActionUzyj
  (:Pressed
    (bind (_poczatek _koniec) (CallFunction|StworzWektor 0.0 5e+02 (Variables|Default|GetCamera1)))
    ;[1 0 0.009181] Rysuj widoczna linie
    (bind (_outhit _returnvalue) (Collision|LineTraceByChannel _poczatek _koniec "TraceTypeQuery2" true 0 "ForDuration"))
    (if _returnvalue
      (Game|Damage|ApplyDamage (.HitActor (Collision|BreakHitResult _outhit)) 0.0 0 0))))

(event Input|ActionEvents|InputActionSkok
  ;[1 1 1] Ruch_Postaci
  ;;[1 1 1] Skok
  (:Pressed
    (Character|Jump)))

(event Input|ActionEvents|InputActionZmien_bron
  ;[1 1 1] Wybieranie broni
  (:Pressed
    (Variables|Default|Setaktualna (Math|Integer|%(Integer) (+ (Variables|Default|Getaktualna) 1) 10))
    (CallFunction|BronZmiana)
    ;[1 0.08657 0] Debug
    (Development|PrintString (Utilities|Array|Get(acopy) (Variables|Default|Getbron_nazwy) (Variables|Default|Getaktualna)))))

(event Input|ActionEvents|InputActionAtak_1
  ;[1 1 1] Atak
  (:Pressed
    (Variables|Default|SetAtak_1_wcisniety true)
    (if (not (Variables|Default|GetPrzeladowuje)) :!label _label
      (bind _opoznienie (CallFunction|Atak1))
      (Utilities|FlowControl|Delay _opoznienie)
      (Variables|Default|SetMozna_strzelac true)
      (if (Utilities|Array|Get(acopy) (Variables|Default|Getbron_automat) (Variables|Default|Getaktualna))
        (if (Variables|Default|GetAtak_1_wcisniety)
          (goto _label)))))
  (:Released
    (Variables|Default|SetAtak_1_wcisniety false)))

(event Input|ActionEvents|InputActionPrzeładuj
  ;[1 1 1] Przeladowanie
  (:Pressed
    (CallFunction|BronPrzeladuj)
    (Utilities|FlowControl|Delay 2.0)
    (Variables|Default|SetPrzeladowuje false)))

(event Input|AxisEvents|InputAxisWidok_Gor_Dol
  (params (AxisValue :type Float%20%28single-precision%29))
  ;[1 1 1] Ruch_Postaci
  ;;[1 1 1] Mysz Ruch
  (Pawn|Input|AddControllerPitchInput AxisValue))

(event Input|AxisEvents|InputAxisRuch_Przod_Tyl
  (params (AxisValue :type Float%20%28single-precision%29))
  ;[1 1 1] Ruch_Postaci
  ;;[1 1 1] Klawiatura Ruch
  (Pawn|Input|AddMovementInput (Math|Vector|GetForwardVector (Class|KismetMathLibrary|MakeRot 0.0 (.Yaw (Class|KismetMathLibrary|BreakRot (Pawn|GetControlRotation :!class /Script/Engine.Pawn))) 0.0)) AxisValue false))

(event Input|AxisEvents|InputAxisRuch_Prawo_Lewo
  (params (AxisValue :type Float%20%28single-precision%29))
  ;[1 1 1] Ruch_Postaci
  ;;[1 1 1] Klawiatura Ruch
  (Pawn|Input|AddMovementInput (Math|Vector|GetRightVector (Class|KismetMathLibrary|MakeRot 0.0 (.Yaw (Class|KismetMathLibrary|BreakRot (Pawn|GetControlRotation :!class /Script/Engine.Pawn))) 0.0)) AxisValue false))

(event Input|AxisEvents|InputAxisWidok_Prawa_Lewa
  (params (AxisValue :type Float%20%28single-precision%29))
  ;[1 1 1] Ruch_Postaci
  ;;[1 1 1] Mysz Ruch
  (Pawn|Input|AddControllerYawInput AxisValue))

(event Input|KeyboardEvents|0
  ;[1 1 1] Wybieranie broni
  (:Pressed
    (Variables|Default|Setaktualna 0)
    (CallFunction|BronZmiana)
    ;[1 0.08657 0] Debug
    (Development|PrintString (Utilities|Array|Get(acopy) (Variables|Default|Getbron_nazwy) (Variables|Default|Getaktualna)))))

(event Input|KeyboardEvents|SpaceBar
  (bind _returnvalue (Game|Player|GetPlayerPawn 0))
  (bind _returnvalue_2 (Transformation|GetActorLocation _returnvalue))
  ;[1 1 1] Hałasowanie
  (:Pressed
    (Audio|PlaySoundatLocation 0 _returnvalue_2)
    (Class|Actor|MakeNoise 1.0 _returnvalue _returnvalue_2)))

(event Input|MouseEvents|LeftMouseButton
  (bind _returnvalue (Game|Player|GetPlayerPawn 0))
  ;[1 1 1] Hałasowanie
  (:Pressed
    (if (not (== 0 1))
      (Class|Actor|MakeNoise 1.0 _returnvalue (Transformation|GetActorLocation _returnvalue)))))

(event Input|KeyboardEvents|1
  ;[1 1 1] Wybieranie broni
  (:Pressed
    (Variables|Default|Setaktualna 1)
    (CallFunction|BronZmiana)
    ;[1 0.08657 0] Debug
    (Development|PrintString (Utilities|Array|Get(acopy) (Variables|Default|Getbron_nazwy) (Variables|Default|Getaktualna)))))

(event Input|KeyboardEvents|2
  ;[1 1 1] Wybieranie broni
  (:Pressed
    (Variables|Default|Setaktualna 2)
    (CallFunction|BronZmiana)
    ;[1 0.08657 0] Debug
    (Development|PrintString (Utilities|Array|Get(acopy) (Variables|Default|Getbron_nazwy) (Variables|Default|Getaktualna)))))

(event Input|KeyboardEvents|3
  ;[1 1 1] Wybieranie broni
  (:Pressed
    (Variables|Default|Setaktualna 3)
    (CallFunction|BronZmiana)
    ;[1 0.08657 0] Debug
    (Development|PrintString (Utilities|Array|Get(acopy) (Variables|Default|Getbron_nazwy) (Variables|Default|Getaktualna)))))

(event Input|KeyboardEvents|4
  ;[1 1 1] Wybieranie broni
  (:Pressed
    (Variables|Default|Setaktualna 4)
    (CallFunction|BronZmiana)
    ;[1 0.08657 0] Debug
    (Development|PrintString (Utilities|Array|Get(acopy) (Variables|Default|Getbron_nazwy) (Variables|Default|Getaktualna)))))

(event Input|KeyboardEvents|5
  ;[1 1 1] Wybieranie broni
  (:Pressed
    (Variables|Default|Setaktualna 5)
    (CallFunction|BronZmiana)
    ;[1 0.08657 0] Debug
    (Development|PrintString (Utilities|Array|Get(acopy) (Variables|Default|Getbron_nazwy) (Variables|Default|Getaktualna)))))

(event Input|KeyboardEvents|6
  ;[1 1 1] Wybieranie broni
  (:Pressed
    (Variables|Default|Setaktualna 6)
    (CallFunction|BronZmiana)
    ;[1 0.08657 0] Debug
    (Development|PrintString (Utilities|Array|Get(acopy) (Variables|Default|Getbron_nazwy) (Variables|Default|Getaktualna)))))

(event Input|KeyboardEvents|7
  ;[1 1 1] Wybieranie broni
  (:Pressed
    (Variables|Default|Setaktualna 7)
    (CallFunction|BronZmiana)
    ;[1 0.08657 0] Debug
    (Development|PrintString (Utilities|Array|Get(acopy) (Variables|Default|Getbron_nazwy) (Variables|Default|Getaktualna)))))

(event Input|KeyboardEvents|8
  ;[1 1 1] Wybieranie broni
  (:Pressed
    (Variables|Default|Setaktualna 8)
    (CallFunction|BronZmiana)
    ;[1 0.08657 0] Debug
    (Development|PrintString (Utilities|Array|Get(acopy) (Variables|Default|Getbron_nazwy) (Variables|Default|Getaktualna)))))

(event Input|KeyboardEvents|9
  ;[1 1 1] Wybieranie broni
  (:Pressed
    (Variables|Default|Setaktualna 9)
    (CallFunction|BronZmiana)
    ;[1 0.08657 0] Debug
    (Development|PrintString (Utilities|Array|Get(acopy) (Variables|Default|Getbron_nazwy) (Variables|Default|Getaktualna)))))

(fn ConstructionScript)

(fn Atak
  (switch Utilities|FlowControl|Switch|SwitchonSpis_Broni "NewEnumerator0"
    (:NewEnumerator1
      (CallFunction|AtakStrzal 0 0.0))))

(fn AtakStrzal
  (params (DzwiekWystrzalu :type Sound%20Base%20Object%20Reference) (Głosnosc :type Float%20%28single-precision%29) (Pociski/strzal :type Integer))
  ;[1 1 1] Strzel przed siebie, pojedynczy
  (Audio|PlaySoundatLocation DzwiekWystrzalu "0, 0, 0" Głosnosc)
  (for _index (range 1 Pociski/strzal)
    (bind (_poczatek _koniec) (CallFunction|StworzWektor (Utilities|Array|Get(acopy) (Variables|Default|Getbron_rozrzut) (Variables|Default|Getaktualna)) (Math|Conversions|ToFloat(Integer) (Utilities|Array|Get(acopy) (Variables|Default|Getbron_zasieg) (Variables|Default|Getaktualna))) (Variables|Default|GetCamera1)))
    ;[1 0 0.009181] Rysuj widoczna linie
    (bind (_outhit _returnvalue) (Collision|LineTraceByChannel _poczatek _koniec "TraceTypeQuery2" true 0 "ForDuration"))
    (if _returnvalue
      (Game|Damage|ApplyDamage (.HitActor (Collision|BreakHitResult _outhit)) 5e+01 0 0))))

(fn BronZmiana
  (bind _bron (Variables|Default|Getbron))
  (bind _aktualna (Variables|Default|Getaktualna))
  (if (== _aktualna 0)
    (LocalVariables|SetWybrana "/Game/Broń/knife.knife")
    (Components|StaticMesh|SetStaticMesh _bron (LocalVariables|GetWybrana) :!label _label)
    (Class|SceneComponent|Attachto _bron (Variables|Default|GetSkeletalMesh1) "E" "KeepRelativeOffset" true)
    (elif (== _aktualna 1)
      (LocalVariables|SetWybrana "/Game/Broń/glock.Glock")
      (goto _label)
      (elif (== _aktualna 2)
        (LocalVariables|SetWybrana "/Game/Broń/dubeltowka.dubeltowka")
        (goto _label)
        (elif (== _aktualna 3)
          (LocalVariables|SetWybrana "/Game/Broń/uzi.Uzi")
          (goto _label)
          (elif (== _aktualna 4)
            (LocalVariables|SetWybrana "/Game/Broń/knife.knife")
            (goto _label)
            (elif (== _aktualna 5)
              (LocalVariables|SetWybrana "/Game/Broń/knife.knife")
              (goto _label)
              (elif (== _aktualna 6)
                (LocalVariables|SetWybrana "/Game/Broń/knife.knife")
                (goto _label)
                (elif (== _aktualna 7)
                  (LocalVariables|SetWybrana "/Game/Broń/knife.knife")
                  (goto _label)
                  (elif (== _aktualna 8)
                    (LocalVariables|SetWybrana "/Game/Broń/knife.knife")
                    (goto _label)
                    (elif (== _aktualna 9)
                      (LocalVariables|SetWybrana "/Game/Broń/knife.knife")
                      (goto _label))))))))))))

(fn BronPrzeladuj
  (bind _ammo_pojemnoscmagazynka (Variables|Default|Getammo_pojemnoscMagazynka))
  (bind _aktualna (Variables|Default|Getaktualna))
  (bind _aktualna_2 (Variables|Default|Getaktualna))
  (bind _aktualna_3 (Variables|Default|Getaktualna))
  (bind _ammo_zaladowane (Variables|Default|Getammo_Zaladowane))
  (bind _skeletalmesh1 (Variables|Default|GetSkeletalMesh1))
  (bind _ammo_torba (Variables|Default|Getammo_torba))
  (bind _aktualna_4 (Variables|Default|Getaktualna))
  (bind _item (Utilities|Array|Get(acopy) _ammo_pojemnoscmagazynka _aktualna))
  (bind _item_2 (Utilities|Array|Get(acopy) _ammo_zaladowane _aktualna_3))
  (bind _item_3 (Utilities|Array|Get(acopy) _ammo_torba _aktualna_4))
  (if (< (Utilities|Array|Get(acopy) (Variables|Default|Getammo_Zaladowane) (Variables|Default|Getaktualna)) (Utilities|Array|Get(acopy) (Variables|Default|Getammo_pojemnoscMagazynka) (Variables|Default|Getaktualna)))
    (if (> (Utilities|Array|Get(acopy) (Variables|Default|Getammo_torba) (Variables|Default|Getaktualna)) 0)
      (Variables|Default|SetPrzeladowuje true)
      (if (== _aktualna_2 0)
        ;[1 1 1] Dzwieki
        (Audio|PlaySoundatLocation "/Game/Audio/Broń/Glock/glock_reload_sound.glock_reload_sound" "0, 0, 0")
        ;[1 1 1] Animacje
        (Components|Animation|PlayAnimation _skeletalmesh1 "/Game/Animations/Reload_Pistol.Reload_Pistol" false)
        (if (> (- (Utilities|Array|Get(acopy) (Variables|Default|Getammo_pojemnoscMagazynka) (Variables|Default|Getaktualna)) _item_2) _item_3) :!label _label
          ;[1 1 1] Przypadek II - ostatnie przeładowanie + warunek
          (Utilities|Array|SetArrayElem (Variables|Default|Getammo_Zaladowane) (Variables|Default|Getaktualna) (+ _item_2 _item_3))
          (Utilities|Array|SetArrayElem (Variables|Default|Getammo_torba) (Variables|Default|Getaktualna) 0)
          (else
            ;[1 1 1] Przypadek I - nieostatnie przeładowanie + DOPEŁNIENIE magazynka
            (Utilities|Array|SetArrayElem (Variables|Default|Getammo_torba) (Variables|Default|Getaktualna) (- (Utilities|Array|Get(acopy) (Variables|Default|Getammo_torba) (Variables|Default|Getaktualna)) (- _item (Utilities|Array|Get(acopy) (Variables|Default|Getammo_Zaladowane) (Variables|Default|Getaktualna)))))
            (Utilities|Array|SetArrayElem (Variables|Default|Getammo_Zaladowane) (Variables|Default|Getaktualna) _item)))
        (elif (== _aktualna_2 1)
          (Audio|PlaySoundatLocation "/Game/Audio/Broń/Glock/glock_reload_sound.glock_reload_sound" "0, 0, 0")
          (Components|Animation|PlayAnimation _skeletalmesh1 "/Game/Animations/Reload_Pistol.Reload_Pistol" false)
          (goto _label)
          (elif (== _aktualna_2 2)
            (Audio|PlaySoundatLocation "/Game/Audio/Broń/Glock/glock_reload_sound.glock_reload_sound" "0, 0, 0")
            (Components|Animation|PlayAnimation _skeletalmesh1 "/Game/Animations/Reload_Pistol.Reload_Pistol" false)
            (goto _label)
            (elif (== _aktualna_2 3)
              (Audio|PlaySoundatLocation "/Game/Audio/Broń/Glock/glock_reload_sound.glock_reload_sound" "0, 0, 0")
              (Components|Animation|PlayAnimation _skeletalmesh1 "/Game/Animations/Reload_Pistol.Reload_Pistol" false)
              (goto _label)
              (elif (== _aktualna_2 4)
                (Audio|PlaySoundatLocation "/Game/Audio/Broń/Glock/glock_reload_sound.glock_reload_sound" "0, 0, 0")
                (Components|Animation|PlayAnimation _skeletalmesh1 "/Game/Animations/Reload_Pistol.Reload_Pistol" false)
                (goto _label)
                (elif (== _aktualna_2 5)
                  (Audio|PlaySoundatLocation "/Game/Audio/Broń/Glock/glock_reload_sound.glock_reload_sound" "0, 0, 0")
                  (Components|Animation|PlayAnimation _skeletalmesh1 "/Game/Animations/Reload_Pistol.Reload_Pistol" false)
                  (goto _label)
                  (elif (== _aktualna_2 6)
                    (Audio|PlaySoundatLocation "/Game/Audio/Broń/Glock/glock_reload_sound.glock_reload_sound" "0, 0, 0")
                    (Components|Animation|PlayAnimation _skeletalmesh1 "/Game/Animations/Reload_Pistol.Reload_Pistol" false)
                    (goto _label)
                    (elif (== _aktualna_2 7)
                      (Audio|PlaySoundatLocation "/Game/Audio/Broń/Glock/glock_reload_sound.glock_reload_sound" "0, 0, 0")
                      (Components|Animation|PlayAnimation _skeletalmesh1 "/Game/Animations/Reload_Pistol.Reload_Pistol" false)
                      (goto _label)
                      (elif (== _aktualna_2 8)
                        (Audio|PlaySoundatLocation "/Game/Audio/Broń/Glock/glock_reload_sound.glock_reload_sound" "0, 0, 0")
                        (Components|Animation|PlayAnimation _skeletalmesh1 "/Game/Animations/Reload_Pistol.Reload_Pistol" false)
                        (goto _label)
                        (elif (== _aktualna_2 9)
                          (Audio|PlaySoundatLocation "/Game/Audio/Broń/Glock/glock_reload_sound.glock_reload_sound" "0, 0, 0")
                          (Components|Animation|PlayAnimation _skeletalmesh1 "/Game/Animations/Reload_Pistol.Reload_Pistol" false)
                          (goto _label)))))))))))
      (else
        (Development|PrintString "Zabrakło amunicji!")))
    (else
      (Development|PrintString "Magazynek pełny!"))))

(fn Atak1
  (bind _strzal_glock (Variables|Default|GetStrzal_glock))
  (bind _aktualna (Variables|Default|Getaktualna))
  ;[1 1 1] Czy można strzelić?
  (if (Variables|Default|GetMozna_strzelac)
    (if (== (Utilities|Array|Get(acopy) (Variables|Default|Getammo_Zaladowane) (Variables|Default|Getaktualna)) 0)
      (Development|PrintString "Magazynek pusty!")
      (else
        ;[1 1 1] Strzal
        (Utilities|Array|SetArrayElem (Variables|Default|Getammo_Zaladowane) (Variables|Default|Getaktualna) (- (Utilities|Array|Get(acopy) (Variables|Default|Getammo_Zaladowane) (Variables|Default|Getaktualna)) 1))
        (Variables|Default|SetMozna_strzelac false)
        (if (== _aktualna 0)
          (CallFunction|AtakStrzal _strzal_glock 0.0 1)
          (return (Utilities|Array|Get(acopy) (Variables|Default|Getbron_sekundy/strzal) (Variables|Default|Getaktualna)))
          (elif (== _aktualna 1)
            (CallFunction|AtakStrzal _strzal_glock 0.2 1)
            (return (Utilities|Array|Get(acopy) (Variables|Default|Getbron_sekundy/strzal) (Variables|Default|Getaktualna)))
            (elif (== _aktualna 2)
              (CallFunction|AtakStrzal _strzal_glock 0.2 8)
              (return (Utilities|Array|Get(acopy) (Variables|Default|Getbron_sekundy/strzal) (Variables|Default|Getaktualna)))
              (elif (== _aktualna 3)
                (CallFunction|AtakStrzal _strzal_glock 0.2 1)
                (return (Utilities|Array|Get(acopy) (Variables|Default|Getbron_sekundy/strzal) (Variables|Default|Getaktualna)))
                (elif (== _aktualna 4)
                  (CallFunction|AtakStrzal _strzal_glock 0.2 1)
                  (return (Utilities|Array|Get(acopy) (Variables|Default|Getbron_sekundy/strzal) (Variables|Default|Getaktualna)))
                  (elif (== _aktualna 5)
                    (CallFunction|AtakStrzal _strzal_glock 0.2 1)
                    (return (Utilities|Array|Get(acopy) (Variables|Default|Getbron_sekundy/strzal) (Variables|Default|Getaktualna)))
                    (elif (== _aktualna 6)
                      (CallFunction|AtakStrzal _strzal_glock 0.2 1)
                      (return (Utilities|Array|Get(acopy) (Variables|Default|Getbron_sekundy/strzal) (Variables|Default|Getaktualna)))
                      (elif (== _aktualna 7)
                        (CallFunction|AtakStrzal _strzal_glock 0.2 1)
                        (return (Utilities|Array|Get(acopy) (Variables|Default|Getbron_sekundy/strzal) (Variables|Default|Getaktualna)))
                        (elif (== _aktualna 8)
                          (CallFunction|AtakStrzal _strzal_glock 0.2 1)
                          (return (Utilities|Array|Get(acopy) (Variables|Default|Getbron_sekundy/strzal) (Variables|Default|Getaktualna)))
                          (elif (== _aktualna 9)
                            (CallFunction|AtakStrzal _strzal_glock 0.2 1)
                            (return (Utilities|Array|Get(acopy) (Variables|Default|Getbron_sekundy/strzal) (Variables|Default|Getaktualna)))))))))))))))))

(fn StworzWektor
  (params (Współczynnik%20rozrzutu :type Float%20%28single-precision%29) (Długość :type Float%20%28single-precision%29) (Target :type Scene%20Component%20Object%20Reference))
  (bind _returnvalue (- 0.0 Współczynnik%20rozrzutu))
  (bind _returnvalue_2 (Transformation|GetWorldLocation Target))
  (bind _returnvalue_3 (Math|Vector|GetForwardVector Target))
  (bind (_x _y _z) (Math|Vector|BreakVector _returnvalue_3))
  (return _returnvalue_2 (+ _returnvalue_2 (* (Math|Vector|MakeVector (+ (Math|Random|RandomFloatinRange _returnvalue Współczynnik%20rozrzutu) _x) (+ (Math|Random|RandomFloatinRange _returnvalue Współczynnik%20rozrzutu) _y) (+ (Math|Random|RandomFloatinRange _returnvalue Współczynnik%20rozrzutu) _z)) Długość))))

(fn AmunicjaGlock
  (bind _ammo_zaladowane (Variables|Default|Getammo_Zaladowane))
  (bind _aktualna (Variables|Default|Getaktualna))
  (bind _item (Utilities|Array|Get(acopy) _ammo_zaladowane _aktualna))
  (if (> _item 0)
    (return _item)))

(fn Hp
  (return (Variables|Default|GetZycie) (Variables|Default|GetMax_Zycie)))

(fn MagazynekGlock
  (bind _ammo_torba (Variables|Default|Getammo_torba))
  (bind _aktualna (Variables|Default|Getaktualna))
  (bind _item (Utilities|Array|Get(acopy) _ammo_torba _aktualna))
  (if (> _item 0)
    (return _item)))